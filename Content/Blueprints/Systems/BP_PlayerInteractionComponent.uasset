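; Player interaction component that tracks the current interactable and switches the owning character in and out of dialogue mode.
; TryInteract sends an Interact message with the owner to the stored interactable, which is assigned through SetCurrentInteractable.
; Entering and exiting dialogue toggles the input mode and mouse cursor and swaps the default and dialogue Enhanced Input mapping contexts.
; Exiting also tells any valid current interactable to show its interaction prompt again.
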(event `self.ReceiveBeginPlay`)

(fn `EnterDialogueMode`
  (bind _ascharacter (cast `Character` (`self.GetOwner`)))
  (bind _asplayer_controller (cast `PlayerController` (`Pawn.GetController` _ascharacter)))
  (`WidgetBlueprintLibrary.SetInputMode_GameAndUIEx` _asplayer_controller null)
  (set `PlayerController.bShowMouseCursor` true _asplayer_controller)
  (bind _returnvalue (pcsubsystem `EnhancedInputLocalPlayerSubsystem` _asplayer_controller))
  (`EnhancedInputSubsystemInterface.RemoveMappingContext` _returnvalue "/Game/Input/IMC_Default.IMC_Default" (struct))
  (`EnhancedInputSubsystemInterface.AddMappingContext` _returnvalue "/Game/Input/IMC_Dialogue.IMC_Dialogue" 0 (struct)))

(fn `ExitDialogueMode`
  (bind _currentinteractable (`self.CurrentInteractable`))
  (bind _ascharacter (cast `Character` (`self.GetOwner`)))
  (bind _asplayer_controller (cast `PlayerController` (`Pawn.GetController` _ascharacter)))
  (`WidgetBlueprintLibrary.SetInputMode_GameOnly` _asplayer_controller)
  (set `PlayerController.bShowMouseCursor` false _asplayer_controller)
  (bind _returnvalue (pcsubsystem `EnhancedInputLocalPlayerSubsystem` _asplayer_controller))
  (`EnhancedInputSubsystemInterface.AddMappingContext` _returnvalue "/Game/Input/IMC_Default.IMC_Default" 0 (struct))
  (`EnhancedInputSubsystemInterface.RemoveMappingContext` _returnvalue "/Game/Input/IMC_Dialogue.IMC_Dialogue" (struct))
  (if (`KismetSystemLibrary.IsValid` _currentinteractable)
    (message `/Game/Blueprints/Systems/BPI_Interactable.SetInteractionPromptVisible` _currentinteractable true)))

(fn `SetCurrentInteractable`
  (params (NewInteractable :type "Actor Object Reference"))
  (set `self.CurrentInteractable` NewInteractable))

(fn `TryInteract`
  (bind _currentinteractable (`self.CurrentInteractable`))
  (if (`KismetSystemLibrary.IsValid` _currentinteractable)
    (message `/Game/Blueprints/Systems/BPI_Interactable.Interact` _currentinteractable (`self.GetOwner`))))