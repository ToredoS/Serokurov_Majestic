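; Dialogue game instance that records the player's choices as flags and decides which dialogue choices are shown.
; Helper functions add, remove and query flags in the ChoicesMade collection.
; ShouldShowChoice always shows choices whose RequiredFlag is None; otherwise it compares the flag's presence to RequireFlagPresent, so a flag can either unlock or hide a choice.
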(fn `AddChoiceFlag`
  (params (FlagName :type Name))
  (`BlueprintSetLibrary.Set_Add` (`self.ChoicesMade`) FlagName))

(fn `HasChoiceFlag`
  (params (FlagName :type Name))
  (returns (bIsSet :type Boolean))
  (return (`BlueprintSetLibrary.Set_Contains` (`self.ChoicesMade`) FlagName)))

(fn `RemoveChoiceFlag`
  (params (FlagName :type Name))
  (`BlueprintSetLibrary.Set_Remove` (`self.ChoicesMade`) FlagName))

(fn `ShouldShowChoice`
  (params (Choice :type "/Game/Data/S_DialogueChoice Structure"))
  (returns (`Return Node` :type Boolean))
  (bind (_choicetext _nextlineid _isexitchoice _requiredflag _requireflagpresent) (break `/Game/Data/S_DialogueChoice` Choice))
  (if (== _requiredflag "None")
    (return true)
    (else
      (bind _bisset (`self.HasChoiceFlag` _requiredflag))
      (return (== _bisset _requireflagpresent)))))